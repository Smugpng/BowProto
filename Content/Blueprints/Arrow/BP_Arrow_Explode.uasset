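; BP_Arrow_Explode is an explosive arrow variant that triggers an explosion on hit.
; On BeginPlay it binds a HIT event to its BPCArrowBalistics component and prints a debug message.
; A hit plays a sound at the arrow's location, then calls the component's ExplosionArrowFunction, which handles the explosion.
; The construction script runs the parent's version and sets a short LifetimeTimer.
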(event Custom|HIT!
  (Audio|PlaySoundatLocation "/Game/Audio/button_fx_avr/fx/delay/button_fx_delay_002_003_cc0_avr.button_fx_delay_002_003_cc0_avr" (Transformation|GetActorLocation) "0, 0, 0" 1.0 1.0 0.0 0 0 0 0)
  (Default|ExplosionArrowFunction (Variables|Default|GetBPC_ArrowBalistics)))

(event EventBeginPlay
  (EventDispatchers|BindEventtoHit (Variables|Default|GetBPC_ArrowBalistics) (delegate Custom|HIT!))
  (Development|PrintString "I am a boom arrow!"))

(fn ConstructionScript
  (|CallParentFunction)
  (Variables|Default|SetLifetime%20Timer 0.5))