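; BP_Arrow is an arrow projectile actor whose flight is driven by a ballistics component.
; On construction it scales the component's speed by a speed multiplier.
; When the component reports a hit, a timer waits out the arrow's lifetime, then a timeline eases the actor's scale before destroying it.
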(event Hit(BPC_ArrowBalistics)
  (Utilities|Time|SetTimerbyEvent (delegate Custom|Destroy%20Arrow) (Variables|Default|GetLifetime%20Timer) false false 0.0 1.24))

(event Custom|Destroy%20Arrow
  (bind _alpha (Timeline|Timeline Play)
    (:Update
      (Transformation|SetActorScale3D (Math|Interpolation|Ease :Function "EaseIn" :Alpha _alpha :A (Transformation|GetActorScale3D))))
    (:Finished
      (Actor|DestroyActor))))

(fn ConstructionScript
  (bind _bpc_arrowbalistics (Variables|Default|GetBPC_ArrowBalistics))
  (Variables|/Game/Blueprints/Arrow/BPC_ArrowBalistics.BPC_ArrowBalistics_C|SetSpeed _bpc_arrowbalistics (* (* (Variables|Default|GetspeedMutiplyer) 2.5) (Variables|/Game/Blueprints/Arrow/BPC_ArrowBalistics.BPC_ArrowBalistics_C|GetSpeed _bpc_arrowbalistics))))