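; Actor component that drives arrow projectile flight and supplies normal, explosive, electric and teleport impact functions.
; Tick moves the owner by manual velocity and gravity, line-tracing each step; hits fire CallHit and BPI_Hittable, while misses expire on a timer.
; Impact functions damage AC_Health at the closest bone, stick arrows to targets, apply blast impulses or repeatedly shock nearby actors.
; The teleport call is disconnected, so that variant behaves like a normal arrow.
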(event Custom|Destroy%20Arrow
  (Actor|DestroyActor (Variables|Default|GetOwning%20Actor)))

(event Custom|Target%20Hit
  (params (Hit%20location :type Vector) (HitActor :type Actor%20Object%20Reference))
  ;[0.15 0.15 0.15 0.5] Inital Hit
  (Variables|HitActor|SetHit%20Location Hit%20location)
  ;[0.15 0.15 0.15 0.5] On hit
  (Variables|HitActor|SetHit%20Actor HitActor)
  (Default|CallHit)
  (CallFunction|CheckforHitFunction)
  (Utilities|Time|SetTimerbyEvent (delegate Custom|Destroy%20Actor) 1e+01))

(event Custom|Electric%20Check
  (Utilities|Time|SetTimerbyEvent (delegate Custom|Shock%20Area) 1.5 true false -1.0))

(event Custom|Shock%20Area
  (bind _owning_actor (Variables|Default|GetOwning%20Actor))
  (bind _returnvalue (Transformation|GetActorLocation _owning_actor))
  (if (Utilities|IsValid _owning_actor)
    (bind (_outhits _returnvalue_2) (Collision|MultiSphereTraceByChannel _returnvalue _returnvalue 4e+02 "TraceTypeQuery3" false (Utilities|Array|MakeArray (Variables|Default|GetOwning%20Actor)) "ForOneFrame" true "(R=1.000000,G=0.000000,B=0.000000,A=1.000000)" "(R=0.000000,G=1.000000,B=0.000000,A=1.000000)" 2.0))
    (if _returnvalue_2
      (for _array_element _outhits
        (Utilities|Array|AddUnique (Variables|HitActor|GetHit%20Actors) (.hitactor _array_element)))
      (for _array_element_2 (Variables|HitActor|GetHit%20Actors)
        (Variables|HitActor|SetHit%20Actor _array_element_2)
        (bind _contains_health_compment_mesh (CallFunction|CheckforDamage))
        (if _contains_health_compment_mesh
          (Rendering|Debug|DrawDebugLine :LineStart (Transformation|GetActorLocation (Variables|Default|GetOwning%20Actor)) :LineEnd (Transformation|GetActorLocation (Variables|HitActor|GetHit%20Actor)) :Duration 0.5)
          (CallFunction|Damage)
          (Default|CallRagdoll (Variables|HitActor|GetHealth%20Component))))
      (Utilities|Array|Clear (Variables|HitActor|GetHit%20Actors)))))

(event Custom|Destroy%20Actor
  ;[0.15 0.15 0.15 0.5] On hit
)

(event EventTick
  (params (DeltaSeconds :type Float%20%28single-precision%29))
  (if (not (Variables|Default|GethasHit?))
    (Variables|Default|SetDelta%20Time DeltaSeconds)
    (Variables|Default|SetStartPos (Transformation|GetActorLocation (Variables|Default|GetOwning%20Actor)))
    (Variables|Default|SetEndPos (+ (Variables|Default|GetStartPos) (* (Variables|Default|GetVelocity) (Variables|Default|GetDelta%20Time))))
    (bind (_outhit _returnvalue) (Collision|LineTraceByChannel (Variables|Default|GetStartPos) (Variables|Default|GetEndPos) "TraceTypeQuery3" false 0 "ForDuration" true "(R=1.000000,G=0.000000,B=0.000000,A=1.000000)" "(R=0.000000,G=1.000000,B=0.000000,A=1.000000)" 0.2))
    (if _returnvalue
      (CallFunction|TargetHit (.impactpoint _outhit) (.hitactor _outhit))
      (else
        ;[0.15 0.15 0.15 0.5] No hit continue on
        (Transformation|SetActorLocation (Variables|Default|GetOwning%20Actor) (Variables|Default|GetEndPos) false false)
        (Variables|Default|SetVelocity (- (Variables|Default|GetVelocity) (* (Math|Vector|MakeVector 0.0 0.0 (* 9.8e+02 1e+01)) (Variables|Default|GetDelta%20Time))))
        (Transformation|SetActorRotation (Variables|Default|GetOwning%20Actor) (Math|Rotator|FindLookatRotation (Variables|Default|GetStartPos) (Variables|Default|GetEndPos)))))))

(event EventBeginPlay
  (Utilities|FlowControl|Sequence
    (:then_0
      (Variables|Default|SetOwning%20Actor (Components|GetOwner)))
    (:then_1
      (Variables|Default|SetVelocity (* (Transformation|GetActorForwardVector (Variables|Default|GetOwning%20Actor)) (Variables|Default|GetSpeed)))
      (Variables|Default|SetStartPos (Transformation|GetActorLocation (Variables|Default|GetOwning%20Actor)))
      (bind _returnvalue (Utilities|Time|SetTimerbyEvent (delegate Custom|Destroy%20Arrow) 2.0))
      (Variables|Default|SetDestroyEvent _returnvalue))))

(fn NormalArrowFunction
  (Utilities|FlowControl|Sequence
    (:then_0
      ;[0.15 0.15 0.15 0.5] Clears Destroy Event and Sets Location
      (Utilities|Time|ClearandInvalidateTimerbyHandle (Variables|Default|GetDestroyEvent))
      (Utilities|FlowControl|DoOnce false
        (:Completed
          (Variables|Default|SethasHit? true)
          (Transformation|SetActorLocation (Variables|Default|GetOwning%20Actor) (Variables|HitActor|GetHit%20Location) false false))))
    (:then_1
      (bind _contains_health_compment_mesh (CallFunction|CheckforDamage))
      (Utilities|FlowControl|Sequence
        (:then_0
          (if _contains_health_compment_mesh
            (CallFunction|Damage)))
        (:then_1
          (CallFunction|AttachtoLocation _contains_health_compment_mesh))))))

(fn CheckforDamage
  (bind _hit_actor (Variables|HitActor|GetHit%20Actor))
  (bind _returnvalue (Actor|GetComponentbyClass _hit_actor "/Game/Blueprints/Entity_Stats/AC_Health.AC_Health_C"))
  ;[0.15 0.15 0.15 0.5] Checks if Actor has Health Component
  (Utilities|IsValid _returnvalue
    (:Is%20Valid
      (bind _output_get (Variables|HitActor|SetHealth%20Component _returnvalue))
      (Variables|HitActor|SetHit%20Mesh (Variables|/Game/Blueprints/Entity_Stats/AC_Health.AC_Health_C|Getmesh _output_get))
      (return true))
    (:Is%20Not%20Valid
      (return false))))

(fn AttachtoLocation
  (params (Contains%20Mesh? :type Boolean))
  (if Contains%20Mesh?
    (Transformation|AttachComponentToComponent (Variables|Default|GetOwning%20Actor) (Variables|HitActor|GetHit%20Mesh) (Variables|HitActor|Getclosest%20bone) "KeepWorld" "KeepWorld" "KeepWorld" true)
    (else
      (Transformation|AttachActorToActor (Variables|Default|GetOwning%20Actor) (Variables|HitActor|GetHit%20Actor) "None" "KeepWorld" "KeepWorld" "KeepWorld" true))))

(fn ExplosionArrowFunction
  (bind _hit_actors (Variables|HitActor|GetHit%20Actors))
  (Utilities|FlowControl|Sequence
    (:then_0
      (Utilities|Time|ClearandInvalidateTimerbyHandle (Variables|Default|GetDestroyEvent))
      (Utilities|FlowControl|DoOnce false
        (:Completed
          (Variables|Default|SethasHit? true))))
    (:then_1
      (bind (_outhits _returnvalue) (Collision|MultiSphereTraceByChannel (Variables|HitActor|GetHit%20Location) (Variables|HitActor|GetHit%20Location) 2.4e+02 "TraceTypeQuery3" false 0 "Persistent"))
      (if _returnvalue
        (for _array_element _outhits
          (bind _output_get (Variables|HitActor|SetHit%20Actor (.hitactor _array_element)))
          (if (not (Utilities|Array|ContainsItem _hit_actors _output_get))
            (Utilities|Array|Add _hit_actors (Variables|HitActor|GetHit%20Actor))
            (bind _contains_health_compment_mesh (CallFunction|CheckforDamage))
            (if _contains_health_compment_mesh
              (bind _output_get_2 (Variables|HitActor|SetHit%20Location (.impactpoint _array_element)))
              (CallFunction|Damage)
              (if (Utilities|Enum|Equal(Enum) (Variables|/Game/Blueprints/Entity_Stats/AC_Health.AC_Health_C|GetActor%20Type (Variables|HitActor|GetHealth%20Component)) "NewEnumerator0")
                (Class|PhysicsObjectBlueprintLibrary|ApplyRadialImpulse (.hitcomponent _array_element) _output_get_2 2e+03 2e+03 "RIF_Constant" false 0.0 true 0.0 1.0))
              (elif (Physics|IsSimulatingPhysics (.hitcomponent _array_element) "None")
                (Physics|AddImpulse (.hitcomponent _array_element) (* (Variables|Default|GetVelocity) 2e+01) "None" false)))))))))

(fn Damage
  (bind _output_get (Variables|HitActor|Setclosest%20bone (.ReturnValue (Class|SkinnedMeshComponent|FindClosestBoneK2 (Variables|HitActor|GetHit%20Mesh) (Variables|HitActor|GetHit%20Location) 0.0))))
  (Default|TakeDamage (Variables|HitActor|GetHealth%20Component) (Variables|Default|GetDamage%20Amount) (Variables|Default|GetOwning%20Actor) _output_get (Variables|Default|GetVelocity) (Variables|HitActor|GetHit%20Location)))

(fn TeleportPlayerFunction
  (Utilities|FlowControl|Sequence
    (:then_0
      (bind _asbp_first_person_character (Utilities|Casting|CastToBP_FirstPersonCharacter (Game|Player|GetPlayerPawn 0))))
    (:then_1
      (CallFunction|NormalArrowFunction))))

(fn ElectricArrowFunction
  (Utilities|FlowControl|Sequence
    (:then_0
      ;[0.15 0.15 0.15 0.5] Clears Destroy Event and Sets Location
      (Utilities|Time|ClearandInvalidateTimerbyHandle (Variables|Default|GetDestroyEvent))
      (Utilities|FlowControl|DoOnce false
        (:Completed
          (Variables|Default|SethasHit? true)
          (Transformation|SetActorLocation (Variables|Default|GetOwning%20Actor) (Variables|HitActor|GetHit%20Location) false false))))
    (:then_1
      (bind _contains_health_compment_mesh (CallFunction|CheckforDamage))
      (CallFunction|AttachtoLocation _contains_health_compment_mesh)
      (Variables|Default|SetVelocity (* (Math|Random|RandomUnitVector) 2e+03))
      (CallFunction|ElectricCheck))))

(fn CheckforHitFunction
  (bind _hit_actor (Variables|HitActor|GetHit%20Actor))
  (if (Utilities|DoesObjectImplementInterface _hit_actor "/Game/Blueprints/Arrow/BPI_Hittable.BPI_Hittable_C")
    (bind _asbpi_hittable (Utilities|Casting|CastToBPI_Hittable _hit_actor))
    (Default|OnHit _asbpi_hittable (Variables|Default|GetOwning%20Actor))))