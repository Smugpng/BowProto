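; BP_Arrow_Grapple is an arrow that teleports the player when it hits.
; On BeginPlay it binds its HIT event to the BPCArrowBalistics component and prints a debug string calling itself a mag arrow.
; The first hit passes a DoOnce, plays a sound at the arrow's location and calls the component's TeleportPlayerFunction, so the teleport logic lives in that component.
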(event Custom|HIT!
  (Utilities|FlowControl|DoOnce false
    (:Completed
      (Audio|PlaySoundatLocation "/Game/Audio/button_fx_avr/fx/delay/button_fx_delay_006_003_cc0_avr.button_fx_delay_006_003_cc0_avr" (Transformation|GetActorLocation) "0, 0, 0" 1.0 1.0 0.0 0 0 0 0)
      (Default|TeleportPlayerFunction (Variables|Default|GetBPC_ArrowBalistics)))))

(event EventBeginPlay
  (EventDispatchers|BindEventtoHit (Variables|Default|GetBPC_ArrowBalistics) (delegate Custom|HIT!))
  (Development|PrintString "I am a mag arrow!"))

(fn ConstructionScript
  (|CallParentFunction))