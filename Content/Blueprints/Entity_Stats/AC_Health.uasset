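; AC_Health is an actor component that tracks an entity's health and handles its damage and death.
; BeginPlay caches GI_GameManager and prints setup warnings; TakeDamage stores hit details, subtracts health, checks death and calls OnHit.
; First death triggers ragdoll and OnDeath, reports killer and victim to the game manager, and, for one actor type, applies a bone impulse from hit velocity.
; Explode separately gives that type a radial impulse.
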(event EventBeginPlay
  (bind _asgi_game_manager (Utilities|Casting|CastToGI_GameManager (Game|GetGameInstance))
    (:then
      (Variables|Default|SetGame%20Manager _asgi_game_manager))
    (:CastFailed
      _))
  (Utilities|FlowControl|Sequence
    (:then_0
      (if (< (Utilities|String|Len (Variables|Stats|GetName)) 0)
        (Development|PrintString (Utilities|String|Append (Utilities|GetDisplayName (Components|GetOwner)) ": has Invalid or no name") true true "(R=0.000000,G=0.660000,B=1.000000,A=1.000000)" 2e+01)))
    (:then_1
      (if (Utilities|Enum|Equal(Enum) (Variables|Stats|GetFaction) "NewEnumerator0")
        (if true
          (Development|PrintString (Utilities|String|Append (Utilities|GetDisplayName (Components|GetOwner)) ": has Invalid or no faction") true true "(R=0.000000,G=0.660000,B=1.000000,A=1.000000)" 2e+01))))
    (:then_2
      (if (== (Variables|Health|Gethealth) 0.0)
        (Development|PrintString (Utilities|String|Append (Utilities|GetDisplayName (Components|GetOwner)) ": has no set health Value") true true "(R=0.000000,G=0.660000,B=1.000000,A=1.000000)" 2e+01)))))

(fn TakeDamage
  (params (Damage%20Amount :type Float%20%28double-precision%29) (Damage%20From :type Actor%20Object%20Reference) (Bone :type Name) (Vel :type Vector) (Hit%20Location :type Vector))
  (Variables|Stats|SetWhoDealtDamage (Utilities|GetDisplayName Damage%20From))
  (bind _output_get (Variables|Health|SetLast%20Damage%20Amount Damage%20Amount))
  (Variables|Health|SetBone Bone)
  (Variables|Health|SetVel Vel)
  (Variables|Health|SetHit%20Location Hit%20Location)
  (bind _output_get_2 (Variables|Health|Sethealth (- (Variables|Health|Gethealth) _output_get)))
  (Development|PrintString (Utilities|String|ToString(Float) _output_get_2))
  (CallFunction|CheckDeath)
  (Default|CallOnHit))

(fn CheckDeath
  (if (and (<= (Variables|Health|Gethealth) 0.0) (not (Variables|Health|GetisDead)))
    (CallFunction|DeathFunc)
    (else
      (return))))

(fn DeathFunc
  (bind _mesh (Variables|Default|Getmesh))
  (Variables|Health|SetisDead true)
  (Utilities|FlowControl|Sequence
    (:then_0
      (Default|CallRagdoll)
      (Default|CallOnDeath)
      (Default|Death (Variables|Default|GetGame%20Manager) (Variables|Stats|GetName) (Variables|Stats|GetCharaterIcon) (Variables|Stats|GetWhoDealtDamage)))
    (:then_1
      (if (Utilities|Enum|Equal(Enum) (Variables|Health|GetActor%20Type) "NewEnumerator0")
        (Physics|SetSimulatePhysics _mesh true)
        (Physics|AddImpulse _mesh (* (Variables|Health|GetVel) 2.0) (Variables|Health|GetBone) false)))))

(fn Explode?
  (params (Origin :type Vector))
  (if (Utilities|Enum|Equal(Enum) (Variables|Health|GetActor%20Type) "NewEnumerator0")
    (Physics|AddRadialImpulse (Variables|Default|Getmesh) Origin 2e+02 2e+02 "RIF_Constant" true)))