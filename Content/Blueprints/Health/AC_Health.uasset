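; Health component that tracks damage and death for its owning actor.
; TakeDamage subtracts damage, stores the hit bone, velocity and location, checks for death and fires a hit notification.
; Death sets a one-time flag, fires ragdoll and death notifications, and for one actor type enables mesh physics with an impulse on the hit bone.
; A separate explosion function applies a radial impulse to that same actor type's mesh.
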(fn TakeDamage
  (params (Damage%20Amount :type Float%20%28double-precision%29) (Damage%20From :type Actor%20Object%20Reference) (Bone :type Name) (Vel :type Vector) (Hit%20Location :type Vector))
  (bind _output_get (Variables|Default|SetLast%20Damage%20Amount Damage%20Amount))
  (Variables|Default|SetBone Bone)
  (Variables|Default|SetVel Vel)
  (Variables|Default|SetHit%20Location Hit%20Location)
  (bind _output_get_2 (Variables|Default|Sethealth (- (Variables|Default|Gethealth) _output_get)))
  (Development|PrintString (Utilities|String|ToString(Float) _output_get_2))
  (CallFunction|CheckDeath)
  (Default|CallOnHit))

(fn CheckDeath
  (if (and (<= (Variables|Default|Gethealth) 0.0) (not (Variables|Default|GetisDead)))
    (CallFunction|DeathFunc)
    (else
      (return))))

(fn DeathFunc
  (bind _mesh (Variables|Default|Getmesh))
  (Variables|Default|SetisDead true)
  (Utilities|FlowControl|Sequence
    (:then_0
      (Default|CallRagdoll)
      (Default|CallOnDeath))
    (:then_1
      (if (Utilities|Enum|Equal(Enum) (Variables|Default|GetActor%20Type) "NewEnumerator0")
        (Physics|SetSimulatePhysics _mesh true)
        (Physics|AddImpulse _mesh (* (Variables|Default|GetVel) 2.0) (Variables|Default|GetBone) false)))))

(fn Explode?
  (params (Origin :type Vector))
  (if (Utilities|Enum|Equal(Enum) (Variables|Default|GetActor%20Type) "NewEnumerator0")
    (Physics|AddRadialImpulse (Variables|Default|Getmesh) Origin 2e+02 2e+02 "RIF_Constant" true)))