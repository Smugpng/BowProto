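; Base enemy drone that chases the player character once spotted and strafes around it at close range.
; PawnSensing locks onto the first player seen, then Tick moves and turns the drone toward it until within AttackRange.
; In range it strafes on a vector blended with the look direction, flipping sides on a random repeating timer.
; AC_Health receives the mesh at construction, and its Ragdoll event destroys the capsule and credits the player's kill once.
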(event OnSeePawn(PawnSensing)
  (params (Pawn :type Pawn%20Object%20Reference))
  (Variables|Default|GetTarget
    (:then)
    (:else
      (bind _asbp_first_person_character (Utilities|Casting|CastToBP_FirstPersonCharacter Pawn))
      (Variables|Default|SetTarget _asbp_first_person_character))))

(event Ragdoll(AC_Health)
  (Components|DestroyComponent (Variables|Collision|GetCapsuleComponent))
  (Utilities|FlowControl|DoOnce false
    (:Completed
      (bind _asbp_first_person_character (Utilities|Casting|CastToBP_FirstPersonCharacter (Game|Player|GetPlayerPawn 0)))
      (Default|OnKill _asbp_first_person_character))))

(event Custom|Change%20Strafe%20Direction
  (bind _isa (Utilities|FlowControl|FlipFlop)
    (:A
      _)
    (:B
      _))
  (Variables|Default|SetStrafe%20Right _isa)
  (Utilities|Time|SetTimerbyEvent (delegate Custom|Change%20Strafe%20Direction) (Math|Random|RandomFloatinRange 2.0 6.0)))

(event EventTick
  (params (DeltaSeconds :type Float%20%28single-precision%29))
  (bind _returnvalue (Transformation|GetActorLocation))
  (bind _target (Variables|Default|GetTarget))
  (bind _returnvalue_2 (Transformation|GetActorLocation _target))
  (bind _returnvalue_3 (+ _returnvalue_2 "0.000000,0.000000,100.000000"))
  (bind _returnvalue_4 (Math|Rotator|FindLookatRotation _returnvalue _returnvalue_3))
  (bind _returnvalue_5 (Math|Rotator|FindLookatRotation _returnvalue _returnvalue_3))
  (bind _target_2 (Variables|Default|GetTarget)
    (:then
      (if (> (Transformation|GetDistanceTo _target_2) (Variables|Default|GetAttack%20Range))
        (Pawn|Input|AddMovementInput (Math|Rotator|GetRotationXVector (Math|Rotator|MakeRotator 0.0 0.0 (.yaw _returnvalue_4))) 1.0 false)
        (Transformation|SetActorRotation (Math|Rotator|Lerp(Rotator) (Transformation|GetActorRotation) (Math|Rotator|MakeRotator 0.0 0.0 (.yaw _returnvalue_4)) 0.5 true))
        (else
          (Pawn|Input|AddMovementInput (Math|Vector|Lerp(Vector) (Math|Vector|GetRightVector _returnvalue_5) (Math|Rotator|GetRotationXVector _returnvalue_5) 0.2) (Math|Float|SelectFloat 0.5 -0.5 (Variables|Default|GetStrafe%20Right)) false))))
    (:else)))

(event EventBeginPlay
  (CallFunction|ChangeStrafeDirection))

(fn ConstructionScript
  (Variables|/Game/Blueprints/Entity_Stats/AC_Health.AC_Health_C|Setmesh (Variables|Default|GetAC_Health) (Variables|Character|GetMesh)))