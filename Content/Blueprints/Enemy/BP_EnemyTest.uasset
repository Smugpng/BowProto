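; BP_EnemyTest is a test enemy that chases the player and reports its death to the player character.
; PawnSensing triggers an AI move when it sees a BP_FirstPersonCharacter.
; The construction script passes the mesh to the AC_Health component, whose Ragdoll event destroys the capsule and calls OnKill on the player once through a DoOnce.
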(event Ragdoll(AC_Health)
  (Components|DestroyComponent (Variables|Collision|GetCapsuleComponent))
  (Utilities|FlowControl|DoOnce false
    (:Completed
      (bind _asbp_first_person_character (Utilities|Casting|CastToBP_FirstPersonCharacter (Game|Player|GetPlayerPawn 0)))
      (Default|OnKill _asbp_first_person_character))))

(event OnSeePawn(PawnSensing)
  (params (Pawn :type Pawn%20Object%20Reference))
  (bind _asbp_first_person_character (Utilities|Casting|CastToBP_FirstPersonCharacter Pawn))
  (AI|AIMoveTo _asbp_first_person_character self "0, 0, 0" 0 5.0 false))

(fn ConstructionScript
  (Variables|/Game/Blueprints/Entity_Stats/AC_Health.AC_Health_C|Setmesh (Variables|Default|GetAC_Health) (Variables|Character|GetMesh)))