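; BP_FloatingDrone is an enemy test drone that hovers and turns to face the first-person player once it sees them.
; Each tick a short downward trace toggles capsule gravity and adds upward impulse to keep it aloft.
; Pawn sensing locks the first seen player as target, and the capsule rotation lerps toward it, or levels out without one.
; On the health component's ragdoll event it destroys the capsule and notifies the player of the kill.
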(event OnSeePawn(PawnSensing)
  (params (Pawn :type Pawn%20Object%20Reference))
  (Variables|Default|GetTarget
    (:then)
    (:else
      (bind _asbp_first_person_character (Utilities|Casting|CastToBP_FirstPersonCharacter Pawn))
      (Variables|Default|SetTarget _asbp_first_person_character))))

(event Ragdoll(AC_Health)
  (Components|DestroyComponent (Variables|Collision|GetCapsuleComponent))
  (Utilities|FlowControl|DoOnce false
    (:Completed
      (bind _asbp_first_person_character (Utilities|Casting|CastToBP_FirstPersonCharacter (Game|Player|GetPlayerPawn 0)))
      (Default|OnKill _asbp_first_person_character))))

(event EventTick
  (params (DeltaSeconds :type Float%20%28single-precision%29))
  (bind _returnvalue (Transformation|GetActorLocation))
  (bind _target (Variables|Default|GetTarget))
  (bind _capsulecomponent (Variables|Collision|GetCapsuleComponent))
  (bind _capsulecomponent_2 (Variables|Collision|GetCapsuleComponent))
  (bind _returnvalue_2 (Transformation|GetWorldLocation _capsulecomponent))
  (bind _returnvalue_3 (Transformation|GetActorLocation _target))
  (bind _returnvalue_4 (+ _returnvalue_3 "0.000000,0.000000,100.000000"))
  (bind _returnvalue_5 (Math|Rotator|FindLookatRotation _returnvalue_2 _returnvalue_4))
  (Utilities|FlowControl|Sequence
    (:then_0
      ;[0.15 0.15 0.15 0.5] Hovering
      (bind _returnvalue_6 (Collision|LineTraceByChannel (Transformation|GetActorLocation) (Math|Vector|MakeVector (.x _returnvalue) (.y _returnvalue) (- (.z _returnvalue) 2e+02)) "TraceTypeQuery1" false 0 "ForOneFrame"))
      (if _returnvalue_6
        (Physics|SetEnableGravity _capsulecomponent_2 false)
        (Physics|AddImpulse (Variables|Collision|GetCapsuleComponent) "0.000000,0.000000,500.000000" "None" false)
        (else
          (Physics|SetEnableGravity _capsulecomponent_2 true))))
    (:then_1
      (Variables|Default|GetTarget
        (:then
          (Variables|Default|SetLookAtRot (Math|Rotator|MakeRotator (.roll _returnvalue_5) (.pitch _returnvalue_5) (.yaw _returnvalue_5))))
        (:else
          (Variables|Default|SetLookAtRot (Math|Rotator|MakeRotator 0.0 0.0 (.yaw (Transformation|GetWorldRotation (Variables|Collision|GetCapsuleComponent))))))))
    (:then_2
      (Transformation|SetWorldRotation (Variables|Collision|GetCapsuleComponent) (Math|Rotator|Lerp(Rotator) (Transformation|GetWorldRotation (Variables|Collision|GetCapsuleComponent)) (Variables|Default|GetLookAtRot) 0.6 true) false false))))

(event EventBeginPlay)

(fn ConstructionScript
  (Variables|/Game/Blueprints/Health/AC_Health.AC_Health_C|Setmesh (Variables|Default|GetAC_Health) (Variables|Character|GetMesh)))