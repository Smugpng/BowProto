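; Physics-driven hover drone enemy that locks onto the first player character it sees and chases it.
; Each tick, four downward traces apply distance-scaled lift, custom damping steadies the capsule, and force plus yaw lerp steer it toward the target.
; AC_Health hits knock it back and cut hover and pursuit for a random few seconds.
; Death stops tick, destroys the capsule and notifies the player of the kill.
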(event OnHit(AC_Health)
  (bind _ac_health (Variables|Default|GetAC_Health))
  (CallFunction|Deactivate)
  (Class|PrimitiveComponent|AddForceatLocation (Variables|Collision|GetCapsuleComponent) (* (Variables|/Game/Blueprints/Health/AC_Health.AC_Health_C|GetVel _ac_health) 5e+02) (Variables|/Game/Blueprints/Health/AC_Health.AC_Health_C|GetHit%20Location _ac_health) "None")
  (Utilities|FlowControl|Delay (Math|Random|RandomFloatinRange 1.0 5.0))
  (CallFunction|Activate))

(event OnSeePawn(PawnSensing)
  (params (Pawn :type Pawn%20Object%20Reference))
  (Variables|Default|GetTarget
    (:then)
    (:else
      (bind _asbp_first_person_character (Utilities|Casting|CastToBP_FirstPersonCharacter Pawn))
      (Variables|Default|SetTarget _asbp_first_person_character))))

(event OnDeath(AC_Health)
  (Actor|Tick|SetActorTickEnabled false)
  (CallFunction|Deactivate)
  (Components|DestroyComponent (Variables|Collision|GetCapsuleComponent))
  (Utilities|FlowControl|DoOnce false
    (:Completed
      (bind _asbp_first_person_character (Utilities|Casting|CastToBP_FirstPersonCharacter (Game|Player|GetPlayerPawn 0)))
      (Default|OnKill _asbp_first_person_character))))

(event Custom|Activate
  (Variables|Hover|SetActive true)
  (Variables|Default|SetisDisabled false))

(event Custom|Deactivate
  (Variables|Hover|SetActive false)
  (Variables|Default|SetisDisabled true))

(event EventTick
  (params (DeltaSeconds :type Float%20%28single-precision%29))
  (Hover|ApplyHoverForce)
  (CallFunction|ApplyLinearDamping)
  (CallFunction|ApplyAngularDamping)
  (Variables|Default|GetTarget
    (:then
      (if (not (Variables|Default|GetisDisabled))
        (bind _returnvalue (CallFunction|MovetoPlayer))
        (CallFunction|LookatPlayer _returnvalue)))
    (:else)))

(event EventBeginPlay
  (ForceCalc|CalcHoverForce)
  (CallFunction|Activate))

(fn ConstructionScript
  (OnStart|InitizlieHover)
  (Variables|/Game/Blueprints/Health/AC_Health.AC_Health_C|Setmesh (Variables|Default|GetAC_Health) (Variables|Character|GetMesh))
  (Variables|Default|SetMax%20Health (Variables|/Game/Blueprints/Health/AC_Health.AC_Health_C|Gethealth (Variables|Default|GetAC_Health))))

(fn InitizlieHover
  (Variables|Components|SetHoverPoints (Utilities|Array|MakeArray (Variables|Default|GetHoverPoint1) (Variables|Default|GetHoverPoint2) (Variables|Default|GetHoverPoint3) (Variables|Default|GetHoverPoint4))))

(fn CalcHoverForce
  (Variables|Hover|SetHover%20Force (* (* (Physics|GetMass (Variables|Collision|GetCapsuleComponent)) (Variables|Hover|GetHover%20Accel)) (Variables|Hover|GetHover%20Multipler))))

(fn ApplyHoverForce
  (bind _capsulecomponent (Variables|Collision|GetCapsuleComponent))
  (if (Variables|Hover|GetActive)
    (for _array_element (Variables|Components|GetHoverPoints)
      (bind (_outhit _returnvalue) (Collision|LineTraceByChannel (Transformation|GetWorldLocation _array_element) (Math|Vector|MakeVector (.X (Math|Vector|BreakVector (Transformation|GetWorldLocation _array_element))) (.Y (Math|Vector|BreakVector (Transformation|GetWorldLocation _array_element))) (- (.Z (Math|Vector|BreakVector (Transformation|GetWorldLocation _array_element))) (Variables|Hover|GetHover%20Distance))) "TraceTypeQuery1" false 0 "ForOneFrame"))
      (if _returnvalue
        (Class|PrimitiveComponent|AddForceatLocation _capsulecomponent (* (Math|Vector|GetUpVector _capsulecomponent) (/ (Variables|Hover|GetHover%20Force) (.Distance (Collision|BreakHitResult _outhit)))) (Transformation|GetWorldLocation _array_element) "None")))))

(fn ApplyLinearDamping
  (Physics|AddForce (Variables|Collision|GetCapsuleComponent) (* (* (Transformation|GetComponentVelocity (Variables|Collision|GetCapsuleComponent)) -1.0) (Variables|Stablizie|GetLin%20Damping)) "None" false))

(fn ApplyAngularDamping
  (bind _capsulecomponent (Variables|Collision|GetCapsuleComponent))
  (Class|PrimitiveComponent|AddTorqueinRadians (Variables|Collision|GetCapsuleComponent) (* (* (Class|PrimitiveComponent|GetPhysicsAngularVelocityinRadians _capsulecomponent "None") -1.0) (* (Class|PrimitiveComponent|GetInertiaTensor _capsulecomponent "None") (Variables|Stablizie|GetAngular%20Damping))) "None" false))

(fn LookatPlayer
  (params (InRot :type Rotator))
  (Transformation|SetActorRotation (Math|Rotator|Lerp(Rotator) (Transformation|GetActorRotation) (Math|Rotator|MakeRotator 0.0 0.0 (.Yaw (Math|Rotator|BreakRotator InRot))) 0.2 true)))

(fn MovetoPlayer
  (bind _returnvalue (Transformation|GetActorLocation))
  (bind _target (Variables|Default|GetTarget))
  (bind _returnvalue_2 (Transformation|GetActorLocation _target))
  (bind _returnvalue_3 (+ _returnvalue_2 "0.000000,0.000000,100.000000"))
  (bind _returnvalue_4 (Math|Rotator|FindLookatRotation _returnvalue _returnvalue_3))
  (if (> (Math|Vector|Distance(Vector) _returnvalue _returnvalue_2) 2e+02)
    (Physics|AddForce (Variables|Collision|GetCapsuleComponent) (* (Math|Rotator|GetRotationXVector _returnvalue_4) 5e+04) "None" false)
    (return _returnvalue_4)))

(fn HealthPercentage
  (return (/ (Variables|/Game/Blueprints/Health/AC_Health.AC_Health_C|Gethealth (Variables|Default|GetAC_Health)) (Variables|Default|GetMax%20Health))))

(fn DegradeStats)