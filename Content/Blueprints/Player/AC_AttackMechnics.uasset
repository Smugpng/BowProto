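; Player attack component for a bow that fires four arrow types: normal, explosive, grapple and mag.
; ChargeBow raises draw strength until full and plays a one-shot sound, while FireBow spawns the current arrow along the first-person camera's aim with that strength as its speed multiplier.
; Firing resets the charge and promotes a randomly queued next arrow; Q swaps current and next, and B prints both for debugging.
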(event Custom|Play%20Charge%20Sound
  (Utilities|FlowControl|DoOnce false
    (:Completed
      (Audio|PlaySound2D "/Game/Audio/button_fx_avr/fx/delay/SC_FullCharged.SC_FullCharged" 1.0 1.0 0.0 0 0))))

(event Custom|Reset%20Sound
  (Utilities|FlowControl|DoOnce false) ; enters at Reset
)

(event EventBeginPlay
  (Variables|Quiver|SetcurrentArrow (Utilities|Enum|ByteToEnumE_ArrowTypes (Math|Conversions|ToByte(Integer) (Math|Random|RandomInteger 3))))
  (CallFunction|NewNextArrow))

(event Input|KeyboardEvents|B
  (params (Key :type Key%20Structure :default "None"))
  (:Pressed
    (Development|PrintString (Utilities|String|Append "current Arrow: " (Utilities|String|EnumtoString (Variables|Quiver|GetcurrentArrow)) ", " "next arrow: " (Utilities|String|EnumtoString (Variables|Quiver|GetnextArrow))))))

(event Input|KeyboardEvents|Q
  (params (Key :type Key%20Structure :default "None"))
  (:Pressed
    (CallFunction|SwapArrows)))

(fn FireBow
  (bind _playercharater (Variables|Default|GetplayerCharater))
  (bind _playercharater_2 (Variables|Default|GetplayerCharater))
  (bind _playercharater_3 (Variables|Default|GetplayerCharater))
  (bind _playercharater_4 (Variables|Default|GetplayerCharater))
  (switch Utilities|FlowControl|Switch|SwitchonE_ArrowTypes (Variables|Quiver|GetcurrentArrow)
    (:NewEnumerator0
      (Game|SpawnActorfromClass "/Game/Blueprints/Arrow/BP_Arrow_Basic.BP_Arrow_Basic_C" (Math|Transform|MakeTransform (Transformation|GetWorldLocation (Variables|/Game/FirstPerson/Blueprints/BP_FirstPersonCharacter.BP_FirstPersonCharacter_C|GetSpawn%20Point _playercharater)) (Transformation|GetWorldRotation (Variables|/Game/FirstPerson/Blueprints/BP_FirstPersonCharacter.BP_FirstPersonCharacter_C|GetFirstPersonCamera _playercharater)) "1.000000,1.000000,1.000000") "Undefined" "MultiplyWithRoot" 0 (Variables|Default|GetdrawStrength) 0))
    (:NewEnumerator1
      (Game|SpawnActorfromClass "/Game/Blueprints/Arrow/BP_Arrow_Explode.BP_Arrow_Explode_C" (Math|Transform|MakeTransform (Transformation|GetWorldLocation (Variables|/Game/FirstPerson/Blueprints/BP_FirstPersonCharacter.BP_FirstPersonCharacter_C|GetSpawn%20Point _playercharater_2)) (Transformation|GetWorldRotation (Variables|/Game/FirstPerson/Blueprints/BP_FirstPersonCharacter.BP_FirstPersonCharacter_C|GetFirstPersonCamera _playercharater_2)) "1.000000,1.000000,1.000000") "Undefined" "MultiplyWithRoot" 0 (Variables|Default|GetdrawStrength) 0))
    (:NewEnumerator2
      (Game|SpawnActorfromClass "/Game/Blueprints/Arrow/BP_Arrow_Grapple.BP_Arrow_Grapple_C" (Math|Transform|MakeTransform (Transformation|GetWorldLocation (Variables|/Game/FirstPerson/Blueprints/BP_FirstPersonCharacter.BP_FirstPersonCharacter_C|GetSpawn%20Point _playercharater_3)) (Transformation|GetWorldRotation (Variables|/Game/FirstPerson/Blueprints/BP_FirstPersonCharacter.BP_FirstPersonCharacter_C|GetFirstPersonCamera _playercharater_3)) "1.000000,1.000000,1.000000") "Undefined" "MultiplyWithRoot" 0 (Variables|Default|GetdrawStrength) 0))
    (:NewEnumerator3
      (Game|SpawnActorfromClass "/Game/Blueprints/Arrow/BP_Arrow_Mag.BP_Arrow_Mag_C" (Math|Transform|MakeTransform (Transformation|GetWorldLocation (Variables|/Game/FirstPerson/Blueprints/BP_FirstPersonCharacter.BP_FirstPersonCharacter_C|GetSpawn%20Point _playercharater_4)) (Transformation|GetWorldRotation (Variables|/Game/FirstPerson/Blueprints/BP_FirstPersonCharacter.BP_FirstPersonCharacter_C|GetFirstPersonCamera _playercharater_4)) "1.000000,1.000000,1.000000") "Undefined" "MultiplyWithRoot" 0 (Variables|Default|GetdrawStrength) 0)))
  (CallFunction|CurrentArrowUsed)
  (CallFunction|ResetBow))

(fn ChargeBow
  (if (>= (Variables|Default|GetdrawStrength) (Variables|Default|GetdrawStrengthMax))
    (CallFunction|PlayChargeSound)
    (else
      (Variables|Default|SetdrawStrength (+ (Variables|Default|GetdrawStrength) 0.05)))))

(fn ResetBow
  (Variables|Default|SetdrawStrength 0.0)
  (CallFunction|ResetSound))

(fn SwapArrows
  (Utilities|FlowControl|Sequence
    (:then_0
      (bind _output_get (LocalVariables|Setcurr (Variables|Quiver|GetcurrentArrow)))
      (bind _output_get_2 (LocalVariables|Setnext (Variables|Quiver|GetnextArrow))))
    (:then_1
      (Variables|Quiver|SetnextArrow _output_get)
      (Variables|Quiver|SetcurrentArrow _output_get_2))))

(fn NewNextArrow
  (Variables|Quiver|SetnextArrow (Utilities|Enum|ByteToEnumE_ArrowTypes (Math|Conversions|ToByte(Integer) (Math|Random|RandomInteger 4)))))

(fn CurrentArrowUsed
  (Variables|Quiver|SetcurrentArrow (Variables|Quiver|GetnextArrow))
  (CallFunction|NewNextArrow))